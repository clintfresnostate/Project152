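; Blue laser robot combatant for grid-based, turn-based combat, with health bar, name display and turn indicator.
; MovetoGridEvent, called from C++, walks the pathway by replaying a timeline per segment, its play rate scaled by distance for constant speed.
; AttackEvent applies random damage and briefly shows a beam; both actions notify the game mode when done.
; Incoming damage spawns floating numbers, updates health and runs a zero-health check.
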(event `self.AttackEvent`
  (bind _returnvalue (`SceneComponent.K2_GetComponentLocation` (`self.BeamSource`)))
  ;[1 0.2446 0.3308] Laser Beam Fire
  (set `self.bIsAttacking` true)
  (set `self.BeamSourceLocation` _returnvalue)
  (bind _returnvalue_2 (`GameplayStatics.SpawnEmitterAtLocation` "/Game/OurContent/GridMaterials/LaserBeam.LaserBeam" _returnvalue))
  (set `self.BeamTargetLocation` (`KismetMathLibrary.MakeVector` (.x (`self.AttackTargetLocation`)) (.y (`self.AttackTargetLocation`)) (.z _returnvalue)))
  (`GameplayStatics.ApplyDamage` (`self.AcquiredTarget`) (`KismetMathLibrary.Conv_IntToDouble` (`KismetMathLibrary.RandomIntegerInRange` (`self.DamageMinStat`) (`self.DamageMaxStat`))) null self)
  (bind _output_get (set `self.Laser` _returnvalue_2))
  (`ParticleSystemComponent.SetBeamSourcePoint` _returnvalue_2 0 (`self.BeamSourceLocation`) 0)
  (`ParticleSystemComponent.SetBeamSourcePoint` _output_get 0 (`self.BeamSourceLocation`) 0)
  (`ParticleSystemComponent.SetBeamEndPoint` _returnvalue_2 0 (`self.BeamTargetLocation`))
  (`ParticleSystemComponent.SetBeamEndPoint` _output_get 0 (`self.BeamTargetLocation`))
  (`SceneComponent.SetWorldScale3D` _returnvalue_2 (5.0 5.0 5.0))
  (bind _asproject_152game_mode_bp (cast `/Game/OurContent/Blueprints/Project_152GameModeBP` (`GameplayStatics.GetGameMode`)))
  (set `self.bChooseAttack` false)
  (`KismetSystemLibrary.Delay` 1.0)
  (`ActorComponent.K2_DestroyComponent` _returnvalue_2)
  (set `self.bIsAttacking` false)
  (set `Project_152GameMode.bDoneWithAttack` true _asproject_152game_mode_bp)
  (`/Engine/EditorBlueprintResources/StandardMacros.DecrementInt` (`self.NumberOfAttacksRemaining`)))

(event `self.MoveToGridEvent`
  (bind _heightoffset (`self.heightoffset`))
  (bind _worldgridref (`self.WorldGridRef`))
  (bind _item (`KismetArrayLibrary.Array_Get` _worldgridref (`KismetArrayLibrary.Array_Get` (`self.PathwayPoints`) (`self.ForLoopVariable`))))
  (bind _item_2 (`KismetArrayLibrary.Array_Get` _worldgridref (`KismetArrayLibrary.Array_Get` (`self.PathwayPoints`) (+ (`self.ForLoopVariable`) 1))))
  (bind _x (.x _item))
  (bind _y (.y _item))
  (bind _x_2 (.x _item_2))
  (bind _y_2 (.y _item_2))
  ;[0 1 1] Function From C++ that carries out actor movement, No real easier way to do this than timeline
  (set `self.bChooseMove` false)
  (set `self.ForLoopVariable` 0)
  (if (< (`self.ForLoopVariable`) (- (`KismetArrayLibrary.Array_Length` (`self.PathwayPoints`)) 1)) :!label _label
    (set `self.bInMovement` true)
    (set `self.X_Direction` (- _x_2 _x))
    (set `self.Y_Direction` (- _y_2 _y))
    (`TimelineComponent.SetPlayRate` (`self.Timeline_0`) (/ (`self.Speed`) (`KismetMathLibrary.VSize` (- _item _item_2))))
    (bind (_direction _newtrack_2) (`Timeline|Timeline_0` :!via `PlayFromStart`)
      (:`Update`
        (`self.K2_SetActorLocation` (`KismetMathLibrary.VLerp` (`KismetMathLibrary.MakeVector` _x _y _heightoffset) (`KismetMathLibrary.MakeVector` _x_2 _y_2 _heightoffset) _newtrack_2)))
      (:`Finished`
        (set `self.bInMovement` false)
        (set `self.ForLoopVariable` (+ (`self.ForLoopVariable`) 1))
        (goto _label)))
    (else
      (bind _asproject_152game_mode_bp (cast `/Game/OurContent/Blueprints/Project_152GameModeBP` (`GameplayStatics.GetGameMode`)))
      (set `Project_152GameMode.bDoneWithMove` true _asproject_152game_mode_bp)
      (`self.UpdatePositionOnGrid` (`self.CombatGrid`))
      (`/Engine/EditorBlueprintResources/StandardMacros.DecrementInt` (`self.NumberOfMovesRemaining`)))))

(event `self.ReceiveBeginPlay`
  (bind _returnvalue (`self.K2_GetActorLocation`))
  (bind _healthstat (`self.HealthStat`))
  ;[1 0.7709 0.002754] Event Begin Play, Set Height Offset and Get Ref to Combat Grid
  (set `self.InitialLocation` _returnvalue)
  (set `self.heightoffset` (.z _returnvalue))
  (bind _outactors (`GameplayStatics.GetAllActorsOfClass` "/Script/Project_152.CombatGrid"))
  (for _array_element _outactors
    (set `self.CombatGrid` _array_element)
    (set `self.WorldGridRef` (`CombatGrid.WorldLocArray` _array_element))
    (break))
  (bind _ashealth_bar (cast `/Game/OurContent/UI/HealthBar` (`WidgetComponent.GetUserWidgetObject` (`self.HealthBar`))))
  (set `/Game/OurContent/UI/HealthBar.Currenthealth` _healthstat _ashealth_bar)
  (set `/Game/OurContent/UI/HealthBar.TotalHealth` _healthstat _ashealth_bar)
  (set `self.Health Bar Ref` _ashealth_bar)
  (bind _asname_display (cast `/Game/OurContent/UI/NameDisplay` (`WidgetComponent.GetUserWidgetObject` (`self.DisplayName`))))
  (set `/Game/OurContent/UI/NameDisplay.DisplayNameTest` (`self.Name`) _asname_display))

(event `self.ReceiveAnyDamage`
  (params (Damage :type "Float (single-precision)") (DamageType :type "DamageType Object Reference") (InstigatedBy :type "Controller Object Reference") (DamageCauser :type "Actor Object Reference"))
  (bind _returnvalue (`KismetMathLibrary.FTrunc` Damage))
  (bind _health_bar_ref (`self.Health Bar Ref`))
  (bind _returnvalue_2 (`|CreateWidget` "/Game/OurContent/UI/FloatingDmg.FloatingDmg_C" null 0 self))
  (`UserWidget.AddToViewport` _returnvalue_2 0)
  (`UserWidget.PlayAnimation` _returnvalue_2 (`/Game/OurContent/UI/FloatingDmg.MoveUP` _returnvalue_2) 0.0 1 "Forward")
  (set `/Game/OurContent/UI/FloatingDmg.DamageText` _returnvalue _returnvalue_2)
  (bind _output_get (set `/Game/OurContent/UI/HealthBar.Currenthealth` (- (`/Game/OurContent/UI/HealthBar.Currenthealth` _health_bar_ref) _returnvalue) _health_bar_ref))
  (set `self.CurrentHealthStat` _output_get)
  (`self.CheckIfHealthIsZero` self))

(event `self.ReceiveTick`
  (params (DeltaSeconds :type "Float (single-precision)"))
  (bind _asproject_152character (cast `Project_152Character` (`Controller.K2_GetPawn` (`GameplayStatics.GetPlayerController` 0))))
  (`self.SetActorRotation` _asproject_152character (`KismetMathLibrary.MakeRotator` (.roll (`KismetMathLibrary.FindLookAtRotation` (`self.K2_GetActorLocation`) (`SceneComponent.K2_GetComponentLocation` (`Project_152Character.SideViewCameraComponent` _asproject_152character)))) (.pitch (`KismetMathLibrary.FindLookAtRotation` (`self.K2_GetActorLocation`) (`SceneComponent.K2_GetComponentLocation` (`Project_152Character.SideViewCameraComponent` _asproject_152character)))) 90.0)))

(event `self.SetTurnIndicatorVisible`
  (bind _turnidicator (`self.TurnIdicator`))
  (if (`SceneComponent.bHiddenInGame` _turnidicator)
    (`SceneComponent.SetHiddenInGame` _turnidicator false false)))

(event `self.SetTurnIndicatorHidden`
  (`SceneComponent.SetHiddenInGame` (`self.TurnIdicator`) true false))

(fn `UserConstructionScript`)