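; Melee robot combatant for grid-based, turn-based combat, though its attack fires a laser beam dealing random stat-ranged damage.
; Movement steps along pathway points with a replayed, speed-scaled Timeline acting as a loop, up to its movement range.
; Finished actions flag the game mode; movement also triggers TakeTurn for a current AI character.
; Also drives health, floating damage, name/XP widgets and turn indicator, hiding itself at zero health.
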(event `self.AttackEvent`
  (bind _returnvalue (`self.K2_GetActorLocation`))
  ;[1 0.2446 0.3308] Laser Beam Fire
  (if (not (`self.bInMovement`))
    (set `self.bIsAttacking` true)
    (set `self.BeamSourceLocation` _returnvalue)
    (bind _returnvalue_2 (`GameplayStatics.SpawnEmitterAtLocation` "/Game/OurContent/GridMaterials/LaserBeam.LaserBeam" _returnvalue))
    (`GameplayStatics.PlaySound2D` "/Game/Assets/Audio/Laser.Laser")
    (set `self.BeamTargetLocation` (`KismetMathLibrary.MakeVector` (.x (`self.AttackTargetLocation`)) (.y (`self.AttackTargetLocation`)) (.z _returnvalue)))
    (`GameplayStatics.ApplyDamage` (`self.AcquiredTarget`) (`KismetMathLibrary.Conv_IntToDouble` (`KismetMathLibrary.RandomIntegerInRange` (`self.DamageMinStat`) (`self.DamageMaxStat`))) null self)
    (bind _output_get (set `self.Laser` _returnvalue_2))
    (`ParticleSystemComponent.SetBeamSourcePoint` _returnvalue_2 0 (`self.BeamSourceLocation`) 0)
    (`ParticleSystemComponent.SetBeamSourcePoint` _output_get 0 (`self.BeamSourceLocation`) 0)
    (`ParticleSystemComponent.SetBeamEndPoint` _returnvalue_2 0 (`self.BeamTargetLocation`))
    (`ParticleSystemComponent.SetBeamEndPoint` _output_get 0 (`self.BeamTargetLocation`))
    (`SceneComponent.SetWorldScale3D` _returnvalue_2 (5.0 5.0 5.0))
    (bind _asproject_152game_mode_bp (cast `/Game/OurContent/Blueprints/Project_152GameModeBP` (`GameplayStatics.GetGameMode`)))
    (set `self.bChooseAttack` false)
    (`KismetSystemLibrary.Delay` 1.0)
    (`ActorComponent.K2_DestroyComponent` _returnvalue_2)
    (set `self.bInMovement` false)
    (set `self.bIsAttacking` false)
    (set `Project_152GameMode.bDoneWithAttack` true _asproject_152game_mode_bp)
    (`/Engine/EditorBlueprintResources/StandardMacros.DecrementInt` (`self.NumberOfAttacksRemaining`))))

(event `self.MoveToGridEvent`
  (bind _heightoffset (`self.heightoffset`))
  (bind _worldgridref (`self.WorldGridRef`))
  (bind _returnvalue (`KismetArrayLibrary.Array_Length` (`self.PathwayPoints`)))
  (bind _item (`KismetArrayLibrary.Array_Get` _worldgridref (`KismetArrayLibrary.Array_Get` (`self.PathwayPoints`) (`self.ForLoopVariable`))))
  (bind _item_2 (`KismetArrayLibrary.Array_Get` _worldgridref (`KismetArrayLibrary.Array_Get` (`self.PathwayPoints`) (+ (`self.ForLoopVariable`) 1))))
  (bind _x (.x _item))
  (bind _y (.y _item))
  (bind _x_2 (.x _item_2))
  (bind _y_2 (.y _item_2))
  ;[0 1 1] Function From C++ that carries out actor movement, No real easier way to do this than timeline
  (if (> _returnvalue 0)
    (set `self.NumberOfTilesCanMove` (`self.MovementRange`))
    (set `self.bChooseMove` false)
    (set `self.ForLoopVariable` 0)
    (if (< (`self.ForLoopVariable`) (- _returnvalue 1)) :!label _label
      (if (> (`self.NumberOfTilesCanMove`) 0)
        (set `self.bInMovement` true)
        (set `self.X_Direction` (- _x_2 _x))
        (set `self.Y_Direction` (- _y_2 _y))
        (`TimelineComponent.SetPlayRate` (`self.Timeline_0`) (/ (`self.Speed`) (`KismetMathLibrary.VSize` (- _item _item_2))))
        (bind (_direction _newtrack_2) (`Timeline|Timeline_0` :!via `PlayFromStart`)
          (:`Update`
            (`self.K2_SetActorLocation` (`KismetMathLibrary.VLerp` (`KismetMathLibrary.MakeVector` _x _y _heightoffset) (`KismetMathLibrary.MakeVector` _x_2 _y_2 _heightoffset) _newtrack_2)))
          (:`Finished`
            (set `self.bInMovement` false)
            (set `self.ForLoopVariable` (+ (`self.ForLoopVariable`) 1))
            (`/Engine/EditorBlueprintResources/StandardMacros.DecrementInt` (`self.NumberOfTilesCanMove`)
              (:`  `
                (goto _label)))))
        (else
          (`self.UpdatePositionOnGrid` (`self.CombatGrid`) :!label _label_2)
          (bind _asproject_152game_mode_bp (cast `/Game/OurContent/Blueprints/Project_152GameModeBP` (`GameplayStatics.GetGameMode`) :!label _label_3))
          (set `Project_152GameMode.bDoneWithMove` true _asproject_152game_mode_bp)
          (`/Engine/EditorBlueprintResources/StandardMacros.DecrementInt` (`self.NumberOfMovesRemaining`)
            (:`  `
              (bind _asproject_152game_mode (cast `Project_152GameMode` (`GameplayStatics.GetGameMode`)))
              (set `self.bInMovement` false)
              (bind _charactersincombat (`Project_152GameMode.CharactersInCombat` _asproject_152game_mode))
              (bind _item_3 (`KismetArrayLibrary.Array_Get` _charactersincombat (mod (`Project_152GameMode.TurnIncrement` _asproject_152game_mode) (`KismetArrayLibrary.Array_Length` _charactersincombat))))
              (if (not (`ParentCombatCharacter.bIsHumanPlayer` _item_3))
                (`self.TakeTurn` _item_3))))))
      (else
        (goto _label_2)))
    (else
      (set `self.bChooseMove` false)
      (set `self.bInMovement` false)
      (goto _label_3))))

(event `self.ReceiveBeginPlay`
  (bind _returnvalue (`self.K2_GetActorLocation`))
  (bind _healthstat (`self.HealthStat`))
  ;[1 0.7709 0.002754] Event Begin Play, Set Height Offset and Get Ref to Combat Grid
  (set `self.InitialLocation` _returnvalue)
  (set `self.heightoffset` (.z _returnvalue))
  (bind _outactors (`GameplayStatics.GetAllActorsOfClass` "/Script/Project_152.CombatGrid"))
  (for _array_element _outactors
    (set `self.CombatGrid` _array_element)
    (set `self.WorldGridRef` (`CombatGrid.WorldLocArray` _array_element))
    (break))
  (bind _ashealth_bar (cast `/Game/OurContent/UI/HealthBar` (`WidgetComponent.GetUserWidgetObject` (`self.HealthBar`))))
  (set `/Game/OurContent/UI/HealthBar.Currenthealth` _healthstat _ashealth_bar)
  (set `/Game/OurContent/UI/HealthBar.TotalHealth` _healthstat _ashealth_bar)
  (set `self.Health Bar Ref` _ashealth_bar)
  (bind _asname_info_experience (cast `/Game/OurContent/UI/NameInfoExperience` (`WidgetComponent.GetUserWidgetObject` (`self.Name Info`))))
  (set `/Game/OurContent/UI/NameInfoExperience.NameString` (`KismetTextLibrary.Conv_TextToString` (`self.Name`)) _asname_info_experience)
  (set `self.NumberOfTilesCanMove` (`self.MovementRange`)))

(event `self.ReceiveAnyDamage`
  (params (Damage :type "Float (single-precision)") (DamageType :type "DamageType Object Reference") (InstigatedBy :type "Controller Object Reference") (DamageCauser :type "Actor Object Reference"))
  (bind _returnvalue (`KismetMathLibrary.FTrunc` Damage))
  (bind _health_bar_ref (`self.Health Bar Ref`))
  (bind _returnvalue_2 (`|CreateWidget` "/Game/OurContent/UI/FloatingDmg.FloatingDmg_C" null 0 self))
  (`UserWidget.AddToViewport` _returnvalue_2 0)
  (`UserWidget.PlayAnimation` _returnvalue_2 (`/Game/OurContent/UI/FloatingDmg.MoveUP` _returnvalue_2) 0.0 1 "Forward")
  (set `/Game/OurContent/UI/FloatingDmg.DamageText` _returnvalue _returnvalue_2)
  (bind _output_get (set `/Game/OurContent/UI/HealthBar.Currenthealth` (- (`/Game/OurContent/UI/HealthBar.Currenthealth` _health_bar_ref) _returnvalue) _health_bar_ref))
  (set `self.CurrentHealthStat` _output_get)
  (bind _returnvalue_3 (`self.CheckIfHealthIsZero` self))
  (if _returnvalue_3
    (`self.SetActorHiddenInGame` true)))

(event `self.ReceiveTick`
  (params (DeltaSeconds :type "Float (single-precision)"))
  (bind _item (`KismetArrayLibrary.Array_Get` (`self.ExperienceBrackets`) (- (`self.Level`) 1)))
  (bind _asproject_152character (cast `Project_152Character` (`Controller.K2_GetPawn` (`GameplayStatics.GetPlayerController` 0))))
  (`self.SetActorRotation` _asproject_152character (`KismetMathLibrary.MakeRotator` (.roll (`KismetMathLibrary.FindLookAtRotation` (`self.K2_GetActorLocation`) (`SceneComponent.K2_GetComponentLocation` (`Project_152Character.SideViewCameraComponent` _asproject_152character)))) (.pitch (`KismetMathLibrary.FindLookAtRotation` (`self.K2_GetActorLocation`) (`SceneComponent.K2_GetComponentLocation` (`Project_152Character.SideViewCameraComponent` _asproject_152character)))) 90.0))
  (bind _asname_info_experience (cast `/Game/OurContent/UI/NameInfoExperience` (`WidgetComponent.GetUserWidgetObject` (`self.Name Info`))))
  (set `/Game/OurContent/UI/NameInfoExperience.ExperienceTotal` (- (`KismetArrayLibrary.Array_Get` (`self.ExperienceBrackets`) (`self.Level`)) _item) _asname_info_experience)
  (set `/Game/OurContent/UI/NameInfoExperience.InputLevel` (`self.Level`) _asname_info_experience)
  (set `/Game/OurContent/UI/NameInfoExperience.ExperienceCurrent` (- (`self.Experience`) _item) _asname_info_experience))

(event `self.SetTurnIndicatorVisible`
  (bind _turnindicator (`self.TurnIndicator`))
  (if (`SceneComponent.bHiddenInGame` _turnindicator)
    (`SceneComponent.SetHiddenInGame` _turnindicator false false)))

(event `self.SetTurnIndicatorHidden`
  (`SceneComponent.SetHiddenInGame` (`self.TurnIndicator`) true false))

(fn `UserConstructionScript`)