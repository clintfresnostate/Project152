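; CombatGridBP is a grid actor, presumably for combat, that lays out an X by Y floor of tiles.
; Its construction script adds one Floor instance per tile, spaced by TileSize and indexed with Y varying fastest, while incrementing Count.
; It also resizes the TileType array to one less than X*Y, but the node that would write tile values is unconnected.
; The event graph holds no gameplay logic.
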(event `self.ReceiveBeginPlay`)

(event `self.ReceiveActorBeginOverlap`
  (params (OtherActor :type "Actor Object Reference")))

(event `self.ReceiveTick`
  (params (DeltaSeconds :type "Float (single-precision)")))

(fn `UserConstructionScript`
  (bind _y (`self.Y`))
  (bind _tilesize (`self.TileSize`))
  (bind _returnvalue (- (* (`self.X`) (`self.Y`)) 1))
  (`KismetArrayLibrary.Array_Resize` (`self.TileType`) _returnvalue)
  (for _index (range (+ _returnvalue 1))
    (`InstancedStaticMeshComponent.AddInstance` (`self.Floor`) (`KismetMathLibrary.Conv_VectorToTransform` (`KismetMathLibrary.MakeVector` (`KismetMathLibrary.Conv_IntToDouble` (* (/ _index _y) _tilesize)) (`KismetMathLibrary.Conv_IntToDouble` (* (mod _index _y) _tilesize)))))
    (set `self.count` (+ (`self.count`) 1))))