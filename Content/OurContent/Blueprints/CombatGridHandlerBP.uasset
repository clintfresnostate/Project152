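; CombatGridHandlerBP builds a combat tile grid and spawns a character onto it.
; The construction script lays out MaxX by MaxY instanced static mesh tiles, spaced by GridTileSize.
; Two seconds after BeginPlay, it spawns one double-scaled ParentCombatCharacterBP at the first WorldLocArray location, using Offset as height, and hands it that array.
; Nothing in these graphs fills WorldLocArray.
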(event `self.ReceiveBeginPlay`
  (bind _worldlocarray (`self.WorldLocArray`))
  (`KismetSystemLibrary.Delay` 2.0)
  (for (_array_element _array_index) _worldlocarray
    (if (== 0 _array_index)
      (bind _returnvalue (`|SpawnActorFromClass` "/Game/OurContent/Blueprints/ParentCombatCharacterBP.ParentCombatCharacterBP_C" (`KismetMathLibrary.Conv_VectorToTransform` (`KismetMathLibrary.MakeVector` (.x _array_element) (.y _array_element) (`self.Offset`))) "AlwaysSpawn" "OverrideRootScale"))
      (`self.SetActorScale3D` _returnvalue (2.0 2.0 2.0))
      (set `ParentCombatCharacter.WorldGridRef` _worldlocarray _returnvalue))))

(event `self.ReceiveActorBeginOverlap`
  (params (OtherActor :type "Actor Object Reference")))

(event `self.ReceiveTick`
  (params (DeltaSeconds :type "Float (single-precision)")))

(fn `UserConstructionScript`
  (bind _gridtilesize (`self.GridTileSize`))
  (bind _maxy (`self.MaxY`))
  (for _index (range (* (`self.MaxX`) (`self.MaxY`)))
    (`InstancedStaticMeshComponent.AddInstance` (`self.InstancedStaticMesh`) (`KismetMathLibrary.MakeTransform` (.location (`KismetMathLibrary.Conv_VectorToTransform` (`KismetMathLibrary.MakeVector` (`KismetMathLibrary.Conv_IntToDouble` (* (/ _index _maxy) _gridtilesize)) (`KismetMathLibrary.Conv_IntToDouble` (* (mod _index _maxy) _gridtilesize))))) (struct) (1.0 1.0 1.0)))))