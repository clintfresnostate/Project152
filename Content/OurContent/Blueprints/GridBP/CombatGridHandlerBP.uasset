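; Combat grid actor that starts a turn-based battle when a character overlaps its trigger.
; Construction builds the tile grid as instanced static meshes.
; On overlap it hides the player, spawns up to three party members from inventory stats, registers them and three preset AI slots with the game mode, then places both sides on spawn tiles and marks occupancy.
; Events clear combat state or toggle grid visibility.
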(event `self.ReceiveBeginPlay`
  (bind _asproject_152game_mode (cast `Project_152GameMode` (`GameplayStatics.GetGameMode`)))
  (set `self.GameModeRef` _asproject_152game_mode))

(event `self.CombatEnterTest.OnComponentBeginOverlap`
  (params (OtherActor :type "Actor Object Reference") (OtherComp :type "PrimitiveComponent Object Reference") (OtherBodyIndex :type Integer) (bFromSweep :type Boolean) (SweepResult :type "HitResult Structure (by ref)"))
  (bind _aicharinventory (`self.AICharInventory`))
  (bind _computerslot1 (`self.ComputerSlot1`))
  (bind _computerslot2 (`self.ComputerSlot2`))
  (bind _computerslot3 (`self.ComputerSlot3`))
  (bind _asproject_152game_mode_bp (cast `/Game/OurContent/Blueprints/Project_152GameModeBP` (`GameplayStatics.GetGameMode`)))
  (set `Project_152GameMode.TurnIncrement` 0 _asproject_152game_mode_bp)
  (if (not (`self.SpawnedCombat?`))
    (set `self.SpawnedCombat?` true)
    (bind _asplayer_character (cast `/Game/OurContent/Blueprints/PlayerCharacter` (`GameplayStatics.GetPlayerCharacter` 0)))
    (`SceneComponent.SetVisibility` (`PaperCharacter.Sprite` _asplayer_character) false false)
    (`PrimitiveComponent.SetCollisionObjectType` (`Character.CapsuleComponent` _asplayer_character) "ECC_Camera")
    (bind _asproject_152character (cast `Project_152Character` OtherActor))
    (`KismetSystemLibrary.Delay` 5.0)
    ;[1 1 1] TEST, Set this during turn handler
    (set `Project_152Character.bMyTurnInCombat` true _asproject_152character)
    (if (not (`Project_152GameMode.bInCombat` (`self.GameModeRef`)))
      (bind _asproject_152character_2 (cast `Project_152Character` (`GameplayStatics.GetPlayerCharacter` 0)))
      (for (_array_element _array_index) (`Project_152Character.ParentCombatCharacterInventoryArray` _asproject_152character_2)
        (switch `int` _array_index
          (:`0`
            (bind (_itemclass _classofcombatchar _itemimage _itemname _actiontext _sellprice _itemid _itemslotindexholder _health _stamina _strength _speed _intelligence _experience) (break `InventoryItemStruct` _array_element))
            (set `self.HumanSlotOne` _classofcombatchar))
          (:`1`
            (set `self.HumanSlotTwo` _classofcombatchar))
          (:`2`
            (set `self.HumanSlotThree` _classofcombatchar)))
        (bind _returnvalue (`|SpawnActorFromClass` _classofcombatchar (`KismetMathLibrary.MakeTransform` (0.0 0.0 60.0)) "AlwaysSpawn" "OverrideRootScale"))
        (set `ParentCombatCharacter.ItemId` _itemid _returnvalue)
        (set `ParentCombatCharacter.HealthStat` _health _returnvalue)
        (set `ParentCombatCharacter.Stamina` _stamina _returnvalue)
        (set `ParentCombatCharacter.Strength` _strength _returnvalue)
        (set `ParentCombatCharacter.SpeedStat` _speed _returnvalue)
        (set `ParentCombatCharacter.Intelligence` _intelligence _returnvalue)
        (set `ParentCombatCharacter.Experience` _experience _returnvalue)
        (`ParentCombatCharacter.UpdateLevelAndExperienceFromTotal` _returnvalue)
        (set `ParentCombatCharacter.bIsHumanPlayer` true _returnvalue)
        (`KismetArrayLibrary.Array_Add` (`Project_152GameMode.CharactersInCombat` (`self.GameModeRef`)) _returnvalue)
        (`KismetArrayLibrary.Array_Add` (`self.PlayerCharInv`) _returnvalue))
      (set `ParentCombatCharacter.bIsHumanPlayer` false _computerslot1)
      (`KismetArrayLibrary.Array_Add` (`Project_152GameMode.CharactersInCombat` (`self.GameModeRef`)) _computerslot1)
      (`KismetArrayLibrary.Array_Add` _aicharinventory _computerslot1)
      (set `ParentCombatCharacter.bIsHumanPlayer` false _computerslot2)
      (`KismetArrayLibrary.Array_Add` (`Project_152GameMode.CharactersInCombat` (`self.GameModeRef`)) _computerslot2)
      (`KismetArrayLibrary.Array_Add` _aicharinventory _computerslot2)
      (set `ParentCombatCharacter.bIsHumanPlayer` false _computerslot3)
      (`KismetArrayLibrary.Array_Add` (`Project_152GameMode.CharactersInCombat` (`self.GameModeRef`)) _computerslot3)
      (`KismetArrayLibrary.Array_Add` _aicharinventory _computerslot3)
      (`|ExecutionSequence`
        (:`then_0`
          (for (_array_element_2 _array_index_2) (`self.PlayerCharInv`)
            (`ParentCombatCharacter.FaceRight` _array_element_2)
            (bind _item (`KismetArrayLibrary.Array_Get` (`self.PlayerSpawnPoints`) _array_index_2))
            (`self.K2_SetActorLocation` _array_element_2 (`KismetMathLibrary.MakeVector` (.x (`KismetArrayLibrary.Array_Get` (`self.WorldLocArray`) _item)) (.y (`KismetArrayLibrary.Array_Get` (`self.WorldLocArray`) _item)) (`self.Offset`)) false false)
            (set `ParentCombatCharacter.CombatGrid` self _array_element_2)
            (bind _output_get (set `ParentCombatCharacter.LastKnownPosition` _item _array_element_2))
            (set `ParentCombatCharacter.IndexOfLocationOnGrid` _item _array_element_2)
            (set `ParentCombatCharacter.WorldGridRef` (`self.WorldLocArray`) _array_element_2)
            (`self.SetActorScale3D` _array_element_2 (1.5 1.5 1.5))
            (if (`ParentCombatCharacter.bIsHumanPlayer` _array_element_2)
              (`KismetArrayLibrary.Array_Set` (`self.GridType`) _output_get 2)
              (else
                (`KismetArrayLibrary.Array_Set` (`self.GridType`) _output_get 3)))))
        (:`then_1`
          (for (_array_element_3 _array_index_3) (`self.AICharInventory`)
            (`ParentCombatCharacter.FaceLeft` _array_element_3)
            (bind _item_2 (`KismetArrayLibrary.Array_Get` (`self.SpawnPoints`) _array_index_3))
            (`self.K2_SetActorLocation` _array_element_3 (`KismetMathLibrary.MakeVector` (.x (`KismetArrayLibrary.Array_Get` (`self.WorldLocArray`) _item_2)) (.y (`KismetArrayLibrary.Array_Get` (`self.WorldLocArray`) _item_2)) (`self.Offset`)) false false)
            (set `ParentCombatCharacter.CombatGrid` self _array_element_3)
            (bind _output_get_2 (set `ParentCombatCharacter.LastKnownPosition` _item_2 _array_element_3))
            (set `ParentCombatCharacter.IndexOfLocationOnGrid` _item_2 _array_element_3)
            (set `ParentCombatCharacter.WorldGridRef` (`self.WorldLocArray`) _array_element_3)
            (`self.SetActorScale3D` _array_element_3 (1.5 1.5 1.5))
            (if (`ParentCombatCharacter.bIsHumanPlayer` _array_element_3)
              (`KismetArrayLibrary.Array_Set` (`self.GridType`) _output_get_2 2)
              (else
                (`KismetArrayLibrary.Array_Set` (`self.GridType`) _output_get_2 3))))
          (set `Project_152GameMode.bInCombat` true (`self.GameModeRef`)))))))

(event `ClearGrid`
  (bind _gridtype (`self.GridType`))
  (`KismetArrayLibrary.Array_Clear` (`self.PlayerCharInv`))
  (`KismetArrayLibrary.Array_Clear` (`self.AICharInventory`))
  (`KismetArrayLibrary.Array_Clear` (`Project_152GameMode.CharactersInCombat` (`self.GameModeRef`)))
  (for (_ _array_index) _gridtype
    (`KismetArrayLibrary.Array_Set` _gridtype _array_index)
    (set `self.SpawnedCombat?` false)))

(event `hide Grid`
  (`SceneComponent.SetVisibility` (`self.InstancedStaticMesh`) false false))

(event `Unhide Grid`
  (`SceneComponent.SetVisibility` (`self.InstancedStaticMesh`) true false))

(fn `UserConstructionScript`
  (bind _gridtilesize (`self.GridTileSize`))
  (bind _maxy (`self.MaxY`))
  (bind _returnvalue (- (* (`self.MaxX`) (`self.MaxY`)) 1))
  (for _index (range (+ _returnvalue 1))
    (`InstancedStaticMeshComponent.AddInstance` (`self.InstancedStaticMesh`) (`KismetMathLibrary.MakeTransform` (.location (`KismetMathLibrary.Conv_VectorToTransform` (`KismetMathLibrary.MakeVector` (`KismetMathLibrary.Conv_IntToDouble` (* (/ _index _maxy) _gridtilesize)) (`KismetMathLibrary.Conv_IntToDouble` (* (mod _index _maxy) _gridtilesize))))) (struct) (1.0 1.0 1.0))))
  (set `self.SECorner` _returnvalue)
  (set `self.NWCorner` 0))