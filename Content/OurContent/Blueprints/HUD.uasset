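; HUD Blueprint that shows a full-screen material overlay while the player character is in its Loading state.
; Each DrawHUD call casts the player character to Project_152Character and checks its Loading flag.
; When the flag is set, it draws the CombatIni material stretched across the current screen dimensions.
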(event `self.ReceiveBeginPlay`)

(event `self.ReceiveDrawHUD`
  (params (SizeX :type Integer) (SizeY :type Integer))
  (bind (_x _y) (`KismetMathLibrary.BreakVector2D` (`self.ScreenDimensions`)))
  (set `self.ScreenDimensions` (`KismetMathLibrary.MakeVector2D` (`KismetMathLibrary.Conv_IntToDouble` SizeX) (`KismetMathLibrary.Conv_IntToDouble` SizeY)))
  (bind _asproject_152character (cast `Project_152Character` (`GameplayStatics.GetPlayerCharacter` 0)))
  (if (`Project_152Character.bLoading` _asproject_152character)
    (`self.DrawMaterialSimple` "/Game/Assets/Materials/CombatIni.CombatIni" 0.0 0.0 _x _y)))

(fn `UserConstructionScript`)