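; HealerBotItem is an inventory item Blueprint for a healer bot that the player can pick up.
; Its Sphere overlap events call SetWithinItemRadius on the PlayerCharacter, passing itself and whether the player is inside the pickup radius.
; A disconnected chain that would stamp ItemInfo with a unique ID from the game mode's incrementing counter never runs.
; The construction script only calls its parent.
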(event `/Game/OurContent/Blueprints/InventoryBlueprints/BlueLaserBotItem.ReceiveBeginPlay`)

(event `self.Sphere.OnComponentBeginOverlap`
  (params (OtherActor :type "Actor Object Reference") (OtherComp :type "PrimitiveComponent Object Reference") (OtherBodyIndex :type Integer) (bFromSweep :type Boolean) (SweepResult :type "HitResult Structure (by ref)"))
  ;[1 1 1] Enables / Disables the picking up of this item based if the player is inside its pickup radius or not
  (bind _asplayer_character (cast `/Game/OurContent/Blueprints/PlayerCharacter` OtherActor))
  (`/Engine/EditorBlueprintResources/StandardMacros.IsValid` _asplayer_character
    (:`Is Valid`
      (`Project_152Character.SetWithinItemRadius` _asplayer_character true self))))

(event `self.ReceiveActorBeginOverlap`
  (params (OtherActor :type "Actor Object Reference")))

(event `self.Sphere.OnComponentEndOverlap`
  (params (OtherActor :type "Actor Object Reference") (OtherComp :type "PrimitiveComponent Object Reference") (OtherBodyIndex :type Integer))
  ;[1 1 1] Enables / Disables the picking up of this item based if the player is inside its pickup radius or not
  (bind _asplayer_character (cast `/Game/OurContent/Blueprints/PlayerCharacter` OtherActor))
  (`Project_152Character.SetWithinItemRadius` _asplayer_character false self))

(event `self.ReceiveTick`
  (params (DeltaSeconds :type "Float (single-precision)")))

(fn `UserConstructionScript`
  (`parent.UserConstructionScript`))