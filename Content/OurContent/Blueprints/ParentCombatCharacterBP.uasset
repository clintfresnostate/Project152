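; Base combat character that moves along a path of cells on the combat grid.
; On BeginPlay it caches the world locations from the first CombatGrid found, stores its starting height and calls MoveToPosition.
; MovetoGridEvent, tied to C++ movement, walks PathwayPoints by replaying a timeline as a loop, lerping between cells at fixed height.
; Play rate scales with segment length for constant speed, while XDirection records horizontal heading.
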(event `self.ReceiveBeginPlay`
  (bind _returnvalue (`self.K2_GetActorLocation`))
  (set `self.Initial Location` _returnvalue)
  (set `self.Offset` (.z _returnvalue))
  (bind _outactors (`GameplayStatics.GetAllActorsOfClass` "/Script/Project_152.CombatGrid"))
  (for _array_element _outactors
    (bind _output_get (set `self.CombatGrid Ref` _array_element))
    (set `self.WorldGridRef` (`CombatGrid.WorldLocArray` _output_get))
    (break))
  (`self.MoveToPosition` 0))

(event `self.MoveToGridEvent`
  (params (InputGridNum :type Integer) (OutputGridNum :type Integer))
  (bind _offset (`self.Offset`))
  (bind _worldgridref (`self.WorldGridRef`))
  (bind _item (`KismetArrayLibrary.Array_Get` _worldgridref (`KismetArrayLibrary.Array_Get` (`self.PathwayPoints`) (`self.LoopCounterForMovement`))))
  (bind _item_2 (`KismetArrayLibrary.Array_Get` _worldgridref (`KismetArrayLibrary.Array_Get` (`self.PathwayPoints`) (+ (`self.LoopCounterForMovement`) 1))))
  (bind _x (.x _item))
  (bind _x_2 (.x _item_2))
  ;[0 1 1] Function From C++ that carries out actor movement, No real easier way to do this than timeline
  (if (< (`self.LoopCounterForMovement`) (- (`KismetArrayLibrary.Array_Length` (`self.PathwayPoints`)) 1)) :!label _label
    (set `self.bInMovement` true)
    (set `self.X_Direction` (- _x_2 _x))
    (`TimelineComponent.SetPlayRate` (`self.Movement`) (/ (`self.Speed_0`) (`KismetMathLibrary.VSize` (- _item _item_2))))
    (bind (_direction _newtrack_2) (`Timeline|Movement` :!via `PlayFromStart`)
      (:`Update`
        (`self.K2_SetActorLocation` (`KismetMathLibrary.VLerp` (`KismetMathLibrary.MakeVector` _x (.y _item) _offset) (`KismetMathLibrary.MakeVector` _x_2 (.y _item_2) _offset) _newtrack_2)))
      (:`Finished`
        (set `self.bInMovement` false)
        (set `self.LoopCounterForMovement` (+ (`self.LoopCounterForMovement`) 1))
        (goto _label)))))

(fn `UserConstructionScript`)