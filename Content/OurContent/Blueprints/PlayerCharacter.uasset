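; Player character Blueprint that handles grid-based combat move selection, item pickup and an inventory menu.
; Each tick it traces under the cursor and sends the hit to the combat grid to get the hovered cell index.
; A left click spawns a selector on that cell and sets it as the first combatant's move target.
; E flags that combatant to choose a move or picks up nearby items; I toggles inventory and cursor.
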(event `Key|E`
  (params (Key :type "Key Structure" :default "AnyKey"))
  (:`Pressed`
    (bind _asproject_152game_mode (cast `Project_152GameMode` (`GameplayStatics.GetGameMode`)))
    (set `ParentCombatCharacter.bChooseMove` true (`KismetArrayLibrary.Array_Get` (`Project_152GameMode.CharactersInCombat` _asproject_152game_mode)))))

(event `Key|LeftMouseButton`
  (params (Key :type "Key Structure" :default "AnyKey"))
  (bind _currentmouselocationindex (`self.CurrentMouseLocationIndex`))
  (:`Pressed`
    (if (`PlayerController.bShowMouseCursor` (`GameplayStatics.GetPlayerController` 0))
      (if (>= (`self.CurrentMouseLocationIndex`) 0)
        (`|SpawnActorFromClass` "/Game/OurContent/GridMaterials/GridSelectorBP.GridSelectorBP_C" (`KismetMathLibrary.Conv_VectorToTransform` (`KismetMathLibrary.MakeVector` (.x (`KismetArrayLibrary.Array_Get` (`CombatGrid.WorldLocArray` (`self.CombatGridRef`)) _currentmouselocationindex)) (.y (`KismetArrayLibrary.Array_Get` (`CombatGrid.WorldLocArray` (`self.CombatGridRef`)) _currentmouselocationindex)) (- (.z (`KismetArrayLibrary.Array_Get` (`CombatGrid.WorldLocArray` (`self.CombatGridRef`)) _currentmouselocationindex)) 105.0))) "AlwaysSpawn" "OverrideRootScale")
        (bind _asproject_152game_mode (cast `Project_152GameMode` (`GameplayStatics.GetGameMode`)))
        (set `ParentCombatCharacter.MoveToChosenPosition` _currentmouselocationindex (`KismetArrayLibrary.Array_Get` (`Project_152GameMode.CharactersInCombat` _asproject_152game_mode)))))))

(event `self.ReceiveTick`
  (params (DeltaSeconds :type "Float (single-precision)"))
  (bind _combatgridref (`self.CombatGridRef`))
  (bind (_hitresult _returnvalue) (`PlayerController.GetHitResultUnderCursorForObjects` (`GameplayStatics.GetPlayerController` 0) (`self.GRID TYPE`) true))
  ;[1 1 1] Event Tick Mouse Functions
  (set `CombatGrid.bMouseIsOnGrid` _returnvalue (`self.CombatGridRef`))
  (bind _output_get (set `/Game/OurContent/Blueprints/GridBP/CombatGridHandlerBP.MouseLoc` (`.Location` (`GameplayStatics.BreakHitResult` _hitresult)) _combatgridref))
  (bind _returnvalue_2 (`CombatGrid.GetGridNum` _combatgridref _output_get))
  (set `self.CurrentMouseLocationIndex` _returnvalue_2))

(event `self.ReceiveBeginPlay`
  ;[1 1 1] Initialize Inventory HUD
  (bind _outactors (`GameplayStatics.GetAllActorsOfClass` "/Game/OurContent/Blueprints/GridBP/CombatGridHandlerBP.CombatGridHandlerBP_C"))
  (for _array_element _outactors
    (bind _output_get (set `self.CombatGridRef` _array_element))
    (break))
  (bind _returnvalue (`|CreateWidget` "/Game/OurContent/UI/Inventory.Inventory_C"))
  (bind _output_get_2 (set `self.InventoryUIRef` _returnvalue))
  (`UserWidget.AddToViewport` _output_get_2 0)
  (`Widget.SetVisibility` (`/Game/OurContent/UI/Inventory.InventoryPanel` _output_get_2) "Hidden"))

(event `Key|I`
  (params (Key :type "Key Structure" :default "AnyKey"))
  (bind _inventoryuiref (`self.InventoryUIRef`))
  (bind _inventorypanel (`/Game/OurContent/UI/Inventory.InventoryPanel` _inventoryuiref))
  ;[1 1 1] Opening Inventory
  (:`Pressed`
    (if (`/Game/OurContent/UI/Inventory.InventoryActive` _inventoryuiref)
      (`Widget.SetVisibility` _inventorypanel "Hidden")
      (set `self.MenuOpen` false)
      (`self.DisableMouseCursor`)
      (set `/Game/OurContent/UI/Inventory.InventoryActive` false _inventoryuiref)
      (`Widget.SetIsEnabled` _inventorypanel false)
      (else
        (`Widget.SetVisibility` _inventorypanel "Visible")
        (set `self.MenuOpen` true)
        (`self.EnableMouseCursor`)
        (set `/Game/OurContent/UI/Inventory.InventoryActive` true _inventoryuiref)
        (`Widget.SetIsEnabled` _inventorypanel true)
        (`self.UpdateInventory`)))))

(event `self.RefreshInventory`
  ;[1 1 1] Update
  (`/Game/OurContent/UI/Inventory.InventoryUpdated_Event` (`self.InventoryUIRef`)))

(event `Key|E`
  (params (Key :type "Key Structure" :default "AnyKey"))
  (bind _focuseditem (`self.FocusedItem`))
  ;[1 1 1] Add to Inventory, Press E
  (:`Pressed`
    (if (`self.bIsWithinItemRange`)
      (`self.GiveItem` (`InventoryItem.ItemInfo` _focuseditem))
      (`self.K2_DestroyActor` _focuseditem)
      (set `self.bIsWithinItemRange` false))))

(fn `DisableMouseCursor`
  (set `PlayerController.bShowMouseCursor` false (`GameplayStatics.GetPlayerController` 0)))

(fn `EnableMouseCursor`
  (set `PlayerController.bShowMouseCursor` true (`GameplayStatics.GetPlayerController` 0)))

(fn `UserConstructionScript`)