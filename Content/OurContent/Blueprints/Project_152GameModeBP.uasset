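; Game mode for turn-based grid combat that handles the end of a battle on a win or a loss.
; BeginPlay caches the level's CombatGrid, and each outcome shows a WinLose widget after a short delay.
; Rewards from the current level's LevelTable row go to ProcessWin, halved on a loss.
; Both outcomes then share cleanup that destroys player and AI characters, clears the grid and resets turn and player combat flags.
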(event `self.ReceiveBeginPlay`
  (bind _outactors (`GameplayStatics.GetAllActorsOfClass` "/Script/Project_152.CombatGrid"))
  (for _array_element _outactors
    (set `self.GridRef` _array_element)
    (break)))

(event `self.ReceiveTick`
  (params (DeltaSeconds :type "Float (single-precision)")))

(event `self.LossExecution`
  (bind _asproject_152game_mode (cast `Project_152GameMode` (`GameplayStatics.GetGameMode`)))
  (set `Project_152GameMode.bInCombat` false _asproject_152game_mode)
  (`KismetSystemLibrary.Delay` 0.2)
  (bind _returnvalue (`|CreateWidget` "/Game/OurContent/UI/WinLose.WinLose_C"))
  ;[1 1 1] WIN/LOSS Condition
  (set `/Game/OurContent/UI/WinLose.win?` false _returnvalue)
  (`UserWidget.AddToViewport` _returnvalue 0)
  (set `self.WinLossUI` _returnvalue)
  (set `self.bInCombat` false)
  (bind _returnvalue_2 (`|GetDataTableRow` "/Game/OurContent/LevelData/LevelTable.LevelTable" (`KismetStringLibrary.Conv_StringToName` (`self.CurrentLevelName`)))
    (:`then`
      (bind (_characters _levelindex _experienceonwin _currencyonwin) (break `/Game/OurContent/LevelData/LevelData` _returnvalue_2))
      (`self.ProcessWin` (/ _experienceonwin 2) (/ _currencyonwin 2))
      (bind _ascombat_grid_handler_bp (cast `/Game/OurContent/Blueprints/GridBP/CombatGridHandlerBP` (`self.GridRef`) :!label _label))
      (for _array_element (`/Game/OurContent/Blueprints/GridBP/CombatGridHandlerBP.PlayerCharInv` _ascombat_grid_handler_bp)
        (`self.K2_DestroyActor` _array_element))
      (for _array_element_2 (`/Game/OurContent/Blueprints/GridBP/CombatGridHandlerBP.AICharInventory` _ascombat_grid_handler_bp)
        (`self.K2_DestroyActor` _array_element_2))
      (bind _ascombat_grid_handler_bp_2 (cast `/Game/OurContent/Blueprints/GridBP/CombatGridHandlerBP` (`self.GridRef`)))
      (`/Game/OurContent/Blueprints/GridBP/CombatGridHandlerBP.ClearGrid` _ascombat_grid_handler_bp_2)
      (bind _asproject_152game_mode_2 (cast `Project_152GameMode` (`GameplayStatics.GetGameMode`)))
      (set `Project_152GameMode.bNextTurn` false _asproject_152game_mode_2)
      (set `Project_152GameMode.bTakeTurn` false _asproject_152game_mode_2)
      (set `Project_152GameMode.bInCombat` false _asproject_152game_mode_2)
      (set `Project_152GameMode.TurnIncrement` 0 _asproject_152game_mode_2)
      (bind _asplayer_character (cast `/Game/OurContent/Blueprints/PlayerCharacter` (`GameplayStatics.GetPlayerCharacter` 0)))
      (set `Project_152Character.bMyTurnInCombat` false _asplayer_character)
      (set `Project_152Character.bPlayerChoseMove` false _asplayer_character)
      (set `Project_152Character.bPlayerChoseAttack` false _asplayer_character))))

(event `self.WinExecution`
  (`KismetSystemLibrary.Delay` 0.2 :!label _label_2)
  (bind _returnvalue (`|CreateWidget` "/Game/OurContent/UI/WinLose.WinLose_C"))
  ;[1 1 1] WIN/LOSS Condition
  (set `/Game/OurContent/UI/WinLose.win?` true _returnvalue)
  (`UserWidget.AddToViewport` _returnvalue 0)
  (set `self.WinLossUI` _returnvalue)
  (set `self.bInCombat` false)
  (bind _returnvalue_2 (`|GetDataTableRow` "/Game/OurContent/LevelData/LevelTable.LevelTable" (`KismetStringLibrary.Conv_StringToName` (`self.CurrentLevelName`)))
    (:`then`
      (bind (_characters _levelindex _experienceonwin _currencyonwin) (break `/Game/OurContent/LevelData/LevelData` _returnvalue_2))
      (`self.ProcessWin` _experienceonwin _currencyonwin)
      (goto _label))))

(event `Win`
  (goto _label_2))

(event `DeleteWidget`
  (`Widget.RemoveFromParent` (`self.WinLossUI`)))

(fn `UserConstructionScript`)