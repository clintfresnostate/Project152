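; Exit trigger sphere that runs a scripted walk-out of the player along negative X.
; On overlap it stops the first TriggerSphere's audio, disables input and sprite updates, and opens a gate.
; Tick feeds the gate, stepping the player's location each frame with a running flipbook until about 1700 units are covered, then restores control.
; End overlap outside combat resets sprite rotation and repeats that distance check; the Timeline movement is unconnected.
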(event `self.ReceiveActorBeginOverlap`
  (params (OtherActor :type "Actor Object Reference")))

(event `/Game/OurContent/Blueprints/TriggerSphere.ReceiveBeginPlay`)

(event `self.Sphere.OnComponentBeginOverlap`
  (params (OtherActor :type "Actor Object Reference") (OtherComp :type "PrimitiveComponent Object Reference") (OtherBodyIndex :type Integer) (bFromSweep :type Boolean) (SweepResult :type "HitResult Structure (by ref)"))
  (bind _returnvalue (`GameplayStatics.GetPlayerController` 0))
  (bind _vector (`self.Vector`))
  (bind _returnvalue_2 (+ _vector (-5.0 0.0 0.0)))
  (bind _outactors (`GameplayStatics.GetAllActorsOfClass` "/Game/OurContent/Blueprints/TriggerSphere.TriggerSphere_C"))
  (for _array_element _outactors
    (`AudioComponent.Stop` (`/Game/OurContent/Blueprints/TriggerSphere.Audio` _array_element))
    (break))
  (bind _asproject_152character (cast `Project_152Character` (`GameplayStatics.GetPlayerCharacter` 0)))
  (bind _returnvalue_3 (`KismetMathLibrary.MakeVector` (.x (`self.K2_GetActorLocation` _asproject_152character)) (.y (`self.K2_GetActorLocation` _asproject_152character)) 100.0))
  (set `self.Vector` _returnvalue_3)
  (set `self.xoffset` _returnvalue_3)
  (set `Project_152Character.bEnableUpdateSprite` false _asproject_152character)
  (`SceneComponent.SetVisibility` (`PaperCharacter.Sprite` _asproject_152character) true false)
  (`self.DisableInput` _asproject_152character _returnvalue)
  (goto _label :!via `Open`))

(event `self.ReceiveTick`
  (params (DeltaSeconds :type "Float (single-precision)"))
  (bind _vector (`self.Vector`))
  (bind _returnvalue (+ _vector (-5.0 0.0 0.0)))
  (`/Engine/EditorBlueprintResources/StandardMacros.Gate` true :!label _label
    (:`Exit`
      (set `self.Vector` _returnvalue)
      (`self.K2_SetActorLocation` (stale `self.Sphere.OnComponentBeginOverlap` _asproject_152character) _returnvalue false false)
      (bind _asplayer_character (cast `/Game/OurContent/Blueprints/PlayerCharacter` (stale `self.Sphere.OnComponentBeginOverlap` _asproject_152character)))
      (`self.SetActorRotation` _asplayer_character (struct))
      (bind _sprite (`PaperCharacter.Sprite` _asplayer_character))
      (`SceneComponent.K2_SetRelativeRotation` _sprite (struct :`Roll` -45.0) false false)
      (`PaperFlipbookComponent.SetFlipbook` _sprite "/Game/OurContent/Animations/Moose_Run.Moose_Run")
      (if (<= (- (.x _vector) (.x (`self.xoffset`))) -1700.0) :!label _label_2
        (`self.EnableInput` (stale `self.Sphere.OnComponentBeginOverlap` _asproject_152character) (`GameplayStatics.GetPlayerController` 0))
        (set `Project_152Character.bEnableUpdateSprite` true (stale `self.Sphere.OnComponentBeginOverlap` _asproject_152character))
        (goto _label :!via `Close`)))))

(event `self.Sphere.OnComponentEndOverlap`
  (params (OtherActor :type "Actor Object Reference") (OtherComp :type "PrimitiveComponent Object Reference") (OtherBodyIndex :type Integer))
  (bind _asplayer_character (cast `/Game/OurContent/Blueprints/PlayerCharacter` (`GameplayStatics.GetPlayerCharacter` 0)))
  (bind _asproject_152game_mode (cast `Project_152GameMode` (`GameplayStatics.GetGameMode`)))
  (if (not (`Project_152GameMode.bInCombat` _asproject_152game_mode))
    (`SceneComponent.K2_SetWorldRotation` (`PaperCharacter.Sprite` _asplayer_character) (struct) false false)
    (goto _label_2)))

(fn `UserConstructionScript`)