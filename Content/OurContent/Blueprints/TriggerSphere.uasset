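; Trigger sphere that opens a level selection screen when the player has combat characters equipped, and prints a warning otherwise.
; It creates the hidden widget on BeginPlay, then on overlap shows it, hides the inventory UI and zeroes walk speed.
; End overlap hides the selection and restores the saved speed.
; A separate Teleport event moves the player to a fixed location, with sounds and a timed Loading flag.
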(event `self.ReceiveActorBeginOverlap`
  (params (OtherActor :type "Actor Object Reference")))

(event `self.ReceiveBeginPlay`
  (bind _returnvalue (`|CreateWidget` "/Game/OurContent/UI/LevelSelection.LevelSelection_C"))
  (`UserWidget.AddToViewport` _returnvalue 0)
  (`Widget.SetVisibility` _returnvalue "Hidden")
  (set `self.LevelSelectRef` _returnvalue))

(event `Teleport`
  (bind _returnvalue (`GameplayStatics.GetPlayerCharacter` 0))
  (bind _asproject_152character (cast `Project_152Character` _returnvalue))
  (set `Project_152Character.bLoading` true _asproject_152character)
  (`self.K2_TeleportTo` :`self` _returnvalue :`DestLocation` (3450.0 472.0 -103.0))
  (`GameplayStatics.PlaySound2D` "/Game/Assets/Audio/LevelSelected.LevelSelected")
  (`AudioComponent.Play` (`self.Audio`) 0.0)
  (`KismetSystemLibrary.Delay` 5.0)
  (set `Project_152Character.bLoading` false _asproject_152character)
  (`GameplayStatics.PlaySound2D` "/Game/Assets/Audio/CombatInitialized.CombatInitialized"))

(event `self.Sphere.OnComponentBeginOverlap`
  (params (OtherActor :type "Actor Object Reference") (OtherComp :type "PrimitiveComponent Object Reference") (OtherBodyIndex :type Integer) (bFromSweep :type Boolean) (SweepResult :type "HitResult Structure (by ref)"))
  (bind _asplayer_character (cast `/Game/OurContent/Blueprints/PlayerCharacter` (`GameplayStatics.GetPlayerCharacter` 0)))
  (if (> (`KismetArrayLibrary.Array_Length` (`Project_152Character.ParentCombatCharacterInventoryArray` _asplayer_character)) 0)
    (bind _charactermovement (`Character.CharacterMovement` _asplayer_character))
    (set `self.Temp` (`CharacterMovementComponent.MaxWalkSpeed` _charactermovement))
    (set `CharacterMovementComponent.MaxWalkSpeed` 0.0 _charactermovement)
    (`Widget.SetVisibility` (`self.LevelSelectRef`) "Visible")
    (set `self.BlockSelection` true)
    (`Widget.SetVisibility` (`/Game/OurContent/Blueprints/PlayerCharacter.InventoryUIRef` _asplayer_character) "Hidden")
    (else
      (`KismetSystemLibrary.PrintString` "No Characters Equipped!!"))))

(event `self.Sphere.OnComponentEndOverlap`
  (params (OtherActor :type "Actor Object Reference") (OtherComp :type "PrimitiveComponent Object Reference") (OtherBodyIndex :type Integer))
  (if (`self.BlockSelection`)
    (`Widget.SetVisibility` (`self.LevelSelectRef`) "Hidden")
    (bind _asplayer_character (cast `/Game/OurContent/Blueprints/PlayerCharacter` (`GameplayStatics.GetPlayerCharacter` 0)))
    (set `CharacterMovementComponent.MaxWalkSpeed` (`self.Temp`) (`Character.CharacterMovement` _asplayer_character))))

(event `self.ReceiveTick`
  (params (DeltaSeconds :type "Float (single-precision)")))

(fn `UserConstructionScript`)